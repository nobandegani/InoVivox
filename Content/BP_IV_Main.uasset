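; Demo Blueprint for the Vivox subsystem, exercising initialization, sign-in, channels, text messaging and transmission from an on-screen panel.
; BeginPlay creates WBP_IV_Main and binds its buttons and Vivox state delegates, which log results and refresh status.
; Keys send test texts, push-to-talk and toggle panel or cursor; EndPlay leaves and signs out.
; Text-receive bindings and 3D positional updates are present but disconnected.
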(event `OnOpenDocumentationClicked_Event`
  (bind _returnvalue (`KismetSystemLibrary.CanLaunchURL` "http://portal.inoland.net/index.php/knowledge_base/view/2"))
  (if _returnvalue
    (`KismetSystemLibrary.LaunchURL` "http://portal.inoland.net/index.php/knowledge_base/view/2")))

(event `OnChannelStateChanged_Event`
  (params (Username :type String) (ChannelName :type String) (ChannelState :type "ConnectionState Enum" :default "Disconnected"))
  (bind _returnvalue (subsystem `VivoxSubsystem`))
  (bind _returnvalue_2 (subsystem `VivoxSubsystem`))
  (bind _username (`self.Username`))
  (bind _username_2 (`self.Username`))
  (bind _channelname (`self.Channelname`))
  ;[1 1 1] Channel State Change log
  (`/InoVivox/UI/WBP_IV_Main.AddChannelStateChangeLog` (`self.WBP_Vivox_Main_Ref`) (`KismetTextLibrary.Conv_StringToText` (`KismetStringLibrary.Concat_StrStr` "user \"" Username "\" with channel \" " ChannelName "\" new state is " (`|GetEnumeratorNameAsString` ChannelState))))
  (`|ExecutionSequence`
    (:`then_0`
      ;[1 1 1] Channel Refresh Button
      (`/InoVivox/UI/WBP_IV_Main.UpdateChannelInfo` (`self.WBP_Vivox_Main_Ref`) (`KismetTextLibrary.Conv_StringToText` (`|GetEnumeratorNameAsString` (`VivoxSubsystem.GetChannelState` _returnvalue_2 _username_2 _channelname))) (`KismetTextLibrary.Conv_StringToText` (`|GetEnumeratorNameAsString` (`VivoxSubsystem.GetChannelType` _returnvalue_2 _username_2 _channelname))) :!label _label))
    (:`then_1`
      ;[1 1 1] Account Refresh Button
      (`/InoVivox/UI/WBP_IV_Main.UpdateAccountInfo` (`self.WBP_Vivox_Main_Ref`) (`KismetTextLibrary.Conv_StringToText` (`|GetEnumeratorNameAsString` (`VivoxSubsystem.GetLoginState` _returnvalue _username))) (`KismetTextLibrary.Conv_StringToText` (`|GetEnumeratorNameAsString` (`VivoxSubsystem.GetTransmissionMode` _returnvalue _username))) (`VivoxSubsystem.GetTransmittingChannels` _returnvalue _username) :!label _label_2))))

(event `OnInitilizeClicked_Event`
  (bind _returnvalue (subsystem `VivoxSubsystem`))
  (bind _wbp_vivox_main_ref (`self.WBP_Vivox_Main_Ref`))
  ;[1 1 1] Initilize Button
  (bind _returnvalue_2 (`VivoxSubsystem.Initilize` (subsystem `VivoxSubsystem`) (`KismetTextLibrary.Conv_TextToString` (`EditableText.Text` (`/InoVivox/UI/WBP_IV_Main.ET_EndPoint` _wbp_vivox_main_ref))) (`KismetTextLibrary.Conv_TextToString` (`EditableText.Text` (`/InoVivox/UI/WBP_IV_Main.ET_Domain` _wbp_vivox_main_ref))) (`KismetTextLibrary.Conv_TextToString` (`EditableText.Text` (`/InoVivox/UI/WBP_IV_Main.ET_Issuer` _wbp_vivox_main_ref))) (`KismetTextLibrary.Conv_TextToString` (`EditableText.Text` (`/InoVivox/UI/WBP_IV_Main.ET_SecretKey` _wbp_vivox_main_ref)))))
  (`TextBlock.SetText` (`/InoVivox/UI/WBP_IV_Main.TB_InitLog` (`self.WBP_Vivox_Main_Ref`)) (`KismetTextLibrary.Conv_StringToText` (`KismetStringLibrary.Concat_StrStr` "initilize is done with error code " (`KismetStringLibrary.Conv_IntToString` _returnvalue_2))))
  (`KismetSystemLibrary.Delay` 0.2)
  ;[1 1 1] Base Refresh Button
  (`/InoVivox/UI/WBP_IV_Main.UpdateBaseInfo` (`self.WBP_Vivox_Main_Ref`) (`KismetTextLibrary.Conv_BoolToText` (`VivoxSubsystem.IsModuleLoaded` _returnvalue)) (`KismetTextLibrary.Conv_BoolToText` (`VivoxSubsystem.IsInitilized` _returnvalue)) :!label _label_3))

(event `Key|N`
  (params (Key :type "Key Structure"))
  (bind _username (`self.Username`))
  ;[1 1 1] Send direct text messages
  (:`Pressed`
    (bind _returnvalue (`VivoxSubsystem.SendDirectText` (subsystem `VivoxSubsystem`) _username (`self.NewFunction` _username) "hello there" (delegate `CustomEvent_2`)))
    (`KismetSystemLibrary.PrintString` (`KismetStringLibrary.Concat_StrStr` "send direct message started with error " (`KismetStringLibrary.Conv_IntToString` _returnvalue)) true true (struct :`G` 0.66 :`B` 1.0 :`A` 1.0) 100.0)))

(event `OnBaseRefreshClicked_Event`
  ;[1 1 1] Base Refresh Button
  (goto _label_3))

(event `OnDirectTextMessageReceived_Event`
  (params (Username :type String) (Text :type String) (Sender :type String) (RecieveTime :type "DateTime Structure"))
  (bind (_year _month _day _hour _minute _second) (`KismetMathLibrary.BreakDateTime` RecieveTime))
  ;[1 1 1] Recieve direct text messages
  (`KismetSystemLibrary.PrintString` (`KismetStringLibrary.Concat_StrStr` "direct message recieved from " Sender "" "" "-----" (`KismetStringLibrary.Concat_StrStr` (`KismetStringLibrary.Conv_IntToString` _hour) ":" (`KismetStringLibrary.Conv_IntToString` _minute) ":" (`KismetStringLibrary.Conv_IntToString` _second)) "-->" Text) true true (struct :`G` 0.66 :`B` 1.0 :`A` 1.0) 100.0))

(event `OnJoinChannelClicked_Event`
  (bind _wbp_vivox_main_ref (`self.WBP_Vivox_Main_Ref`))
  ;[1 1 1] JoinChannel button
  (set `self.Channelname` (`KismetTextLibrary.Conv_TextToString` (`EditableText.GetText` (`/InoVivox/UI/WBP_IV_Main.ET_ChannelName` _wbp_vivox_main_ref))))
  (bind _returnvalue (`VivoxSubsystem.JoinChannel` (subsystem `VivoxSubsystem`) (`self.Username`) (`self.Channelname`) (select `int` (`ComboBoxString.GetSelectedIndex` (`/InoVivox/UI/WBP_IV_Main.CBS_ChannelType` _wbp_vivox_main_ref)) :`0` "NonPositional" :`1` "Positional" :`2` "Echo" :!type "ChannelType Enum") (make `InoChannel3DProperties` 2700) (select `ECheckBoxState` (`CheckBox.GetCheckedState` (`/InoVivox/UI/WBP_IV_Main.CB_ConnectAudio` _wbp_vivox_main_ref)) :`Checked` true) (select `ECheckBoxState` (`CheckBox.GetCheckedState` (`/InoVivox/UI/WBP_IV_Main.CB_ConnectText` _wbp_vivox_main_ref)) :`Checked` true) (select `ECheckBoxState` (`CheckBox.GetCheckedState` (`/InoVivox/UI/WBP_IV_Main.CB_SwitchTransmission` _wbp_vivox_main_ref)) :`Checked` true) (`KismetMathLibrary.MakeTimespan` 1) (delegate `CustomEvent_0`)))
  (`TextBlock.SetText` (`/InoVivox/UI/WBP_IV_Main.TB_ChannelLog` (`self.WBP_Vivox_Main_Ref`)) (`KismetTextLibrary.Conv_StringToText` (`KismetStringLibrary.Concat_StrStr` "join channel is started with error code " (`KismetStringLibrary.Conv_IntToString` _returnvalue))))
  (goto _label))

(event `CustomEvent_2`
  (params (VivoxError :type Integer))
  ;[1 1 1] Send direct text messages
  (`KismetSystemLibrary.PrintString` (`KismetStringLibrary.Concat_StrStr` "send direct message completed with error " (`KismetStringLibrary.Conv_IntToString` VivoxError)) true true (struct :`G` 0.66 :`B` 1.0 :`A` 1.0) 100.0))

(event `OnLoginStateChanged_Event`
  (params (Username :type String) (LoginState :type "LoginState Enum" :default "LoggedOut"))
  ;[1 1 1] Login State Change
  (`/InoVivox/UI/WBP_IV_Main.AddLoginStateChangeLog` (`self.WBP_Vivox_Main_Ref`) (`KismetTextLibrary.Conv_StringToText` (`KismetStringLibrary.Concat_StrStr` "user \"" Username "\" new state is " (`|GetEnumeratorNameAsString` LoginState))))
  (goto _label_2))

(event `CustomEvent_0`
  (params (VivoxError :type Integer))
  ;[1 1 1] JoinChannel button
  (`TextBlock.SetText` (`/InoVivox/UI/WBP_IV_Main.TB_ChannelLog` (`self.WBP_Vivox_Main_Ref`)) (`KismetTextLibrary.Conv_StringToText` (`KismetStringLibrary.Concat_StrStr` "join channel is completed with error code " (`KismetStringLibrary.Conv_IntToString` VivoxError))))
  (goto _label))

(event `self.ReceiveBeginPlay`
  (bind _returnvalue (`GameplayStatics.GetPlayerController` 0))
  ;[1 1 1] Comment
  (bind _returnvalue_2 (`|CreateWidget` "/InoVivox/UI/WBP_IV_Main.WBP_IV_Main_C"))
  (bind _output_get (set `self.WBP_Vivox_Main_Ref` _returnvalue_2))
  (`UserWidget.AddToViewport` _output_get 0)
  (set `PlayerController.bShowMouseCursor` true _returnvalue)
  (`WidgetBlueprintLibrary.SetInputMode_GameAndUIEx` _returnvalue _output_get "DoNotLock" false)
  (`|ExecutionSequence`
    (:`then_0`
      (`|ExecutionSequence`
        (:`then_0`
          ;[1 1 1] Initilize Button
          (add `/InoVivox/UI/WBP_IV_Main.OnInitilizeClicked` (`self.WBP_Vivox_Main_Ref`) (delegate `OnInitilizeClicked_Event`)))
        (:`then_1`
          ;[1 1 1] Base Refresh Button
          (add `/InoVivox/UI/WBP_IV_Main.OnBaseRefreshClicked` (`self.WBP_Vivox_Main_Ref`) (delegate `OnBaseRefreshClicked_Event`)))
        (:`then_2`
          ;[1 1 1] Login State Change
          (add `VivoxSubsystem.OnLoginStateChanged` (subsystem `VivoxSubsystem`) (delegate `OnLoginStateChanged_Event`)))
        (:`then_3`
          ;[1 1 1] Signin Clicked
          (add `/InoVivox/UI/WBP_IV_Main.OnSigninClicked` (`self.WBP_Vivox_Main_Ref`) (delegate `OnSigninClicked_Event`)))
        (:`then_4`
          ;[1 1 1] Account Refresh Button
          (add `/InoVivox/UI/WBP_IV_Main.OnAccountRefreshClicked` (`self.WBP_Vivox_Main_Ref`) (delegate `OnAccountRefreshClicked_Event`)))
        (:`then_5`
          ;[1 1 1] Signout
          (add `/InoVivox/UI/WBP_IV_Main.OnSignoutClicked` (`self.WBP_Vivox_Main_Ref`) (delegate `OnSignoutClicked_Event`)))))
    (:`then_1`
      (`|ExecutionSequence`
        (:`then_0`
          ;[1 1 1] Channel State Change log
          (add `VivoxSubsystem.OnChannelStateChanged` (subsystem `VivoxSubsystem`) (delegate `OnChannelStateChanged_Event`)))
        (:`then_1`
          ;[1 1 1] JoinChannel button
          (add `/InoVivox/UI/WBP_IV_Main.OnJoinChannelClicked` (`self.WBP_Vivox_Main_Ref`) (delegate `OnJoinChannelClicked_Event`)))
        (:`then_2`
          ;[1 1 1] Channel Refresh Button
          (add `/InoVivox/UI/WBP_IV_Main.OnChannelRefreshClicked` (`self.WBP_Vivox_Main_Ref`) (delegate `OnChannelRefreshClicked_Event`)))
        (:`then_3`
          ;[1 1 1] Leave Channel
          (add `/InoVivox/UI/WBP_IV_Main.OnLeaveChannelClicked` (`self.WBP_Vivox_Main_Ref`) (delegate `OnLeaveChannelClicked_Event`)))))
    (:`then_2`
      (`|ExecutionSequence`
        (:`then_0`
          (add `/InoVivox/UI/WBP_IV_Main.OnOpenDocumentationClicked` (`self.WBP_Vivox_Main_Ref`) (delegate `OnOpenDocumentationClicked_Event`)))))))

(event `Key|B`
  (params (Key :type "Key Structure"))
  ;[1 1 1] SendTextMessage
  (:`Pressed`
    (bind _returnvalue (`VivoxSubsystem.SendChannelText` (subsystem `VivoxSubsystem`) (`self.Username`) (`self.Channelname`) "hello" (delegate `CustomEvent_1`)))
    (`KismetSystemLibrary.PrintString` (`KismetStringLibrary.Concat_StrStr` "send text started with error " (`KismetStringLibrary.Conv_IntToString` _returnvalue)) true true (struct :`G` 0.66 :`B` 1.0 :`A` 1.0) 100.0)))

(event `OnChannelTextMessageReceived_Event`
  (params (Username :type String) (ChannelName :type String) (Text :type String) (Sender :type String) (RecieveTime :type "DateTime Structure"))
  (bind (_year _month _day _hour _minute _second) (`KismetMathLibrary.BreakDateTime` RecieveTime))
  ;[1 1 1] OnMessageRecieved
  (`KismetSystemLibrary.PrintString` (`KismetStringLibrary.Concat_StrStr` "message recieved from " Sender " in channel " ChannelName "-----" (`KismetStringLibrary.Concat_StrStr` (`KismetStringLibrary.Conv_IntToString` _hour) ":" (`KismetStringLibrary.Conv_IntToString` _minute) ":" (`KismetStringLibrary.Conv_IntToString` _second)) "-->" Text) true true (struct :`G` 0.66 :`B` 1.0 :`A` 1.0) 100.0))

(event `OnDirectTextMessageReceived_Event_0`
  (params (Username :type String) (Text :type String) (Sender :type String) (RecieveTime :type "DateTime Structure")))

(event `OnChannelStateChanged_Event_0`
  (params (Username :type String) (ChannelName :type String) (ChannelState :type "ConnectionState Enum" :default "Disconnected")))

(event `OnSigninClicked_Event`
  ;[1 1 1] Signin Clicked
  (set `self.Username` (`KismetTextLibrary.Conv_TextToString` (`EditableText.GetText` (`/InoVivox/UI/WBP_IV_Main.ET_Username` (`self.WBP_Vivox_Main_Ref`)))))
  (bind _returnvalue (`VivoxSubsystem.SignIn` (subsystem `VivoxSubsystem`) (`self.Username`) "" (`|MakeArray`) (`KismetMathLibrary.MakeTimespan` 15) true (delegate `CustomEvent_3`)))
  (`TextBlock.SetText` (`/InoVivox/UI/WBP_IV_Main.TB_AccountLog` (`self.WBP_Vivox_Main_Ref`)) (`KismetTextLibrary.Conv_StringToText` (`KismetStringLibrary.Concat_StrStr` "signin is started with error code " (`KismetStringLibrary.Conv_IntToString` _returnvalue))))
  (goto _label_2))

(event `CustomEvent_1`
  (params (VivoxError :type Integer))
  ;[1 1 1] SendTextMessage
  (`KismetSystemLibrary.PrintString` (`KismetStringLibrary.Concat_StrStr` "send text completed with error " (`KismetStringLibrary.Conv_IntToString` VivoxError)) true true (struct :`G` 0.66 :`B` 1.0 :`A` 1.0) 100.0))

(event `Key|N`
  (params (Key :type "Key Structure"))
  (bind _returnvalue (`GameplayStatics.GetPlayerController` 0))
  ;[1 1 1] Toggle show mouse cursor
  (:`Pressed`
    (if (`PlayerController.bShowMouseCursor` _returnvalue)
      (set `PlayerController.bShowMouseCursor` false _returnvalue)
      (else
        (set `PlayerController.bShowMouseCursor` true _returnvalue)))))

(event `OnChannelTextMessageReceived_Event_0`
  (params (Username :type String) (ChannelName :type String) (Text :type String) (Sender :type String) (RecieveTime :type "DateTime Structure")))

(event `OnLoginStateChanged_Event_0`
  (params (Username :type String) (LoginState :type "LoginState Enum" :default "LoggedOut")))

(event `CustomEvent_3`
  (params (VivoxError :type Integer))
  ;[1 1 1] Signin Clicked
  (`TextBlock.SetText` (`/InoVivox/UI/WBP_IV_Main.TB_AccountLog` (`self.WBP_Vivox_Main_Ref`)) (`KismetTextLibrary.Conv_StringToText` (`KismetStringLibrary.Concat_StrStr` "signin is completed with error code " (`KismetStringLibrary.Conv_IntToString` VivoxError))))
  (goto _label_2))

(event `OnChannelRefreshClicked_Event`
  ;[1 1 1] Channel Refresh Button
  (goto _label))

(event `Key|M`
  (params (Key :type "Key Structure"))
  (bind _wbp_vivox_main_ref (`self.WBP_Vivox_Main_Ref`))
  ;[1 1 1] Comment
  (:`Pressed`
    (`/Engine/EditorBlueprintResources/StandardMacros.FlipFlop`
      (:`A`
        (`Widget.RemoveFromParent` _wbp_vivox_main_ref))
      (:`B`
        (`UserWidget.AddToViewport` _wbp_vivox_main_ref 0)))))

(event `self.ReceiveTick`
  (params (DeltaSeconds :type "Float (single-precision)"))
  ;[1 1 1] Update3dPositional
)

(event `OnAccountRefreshClicked_Event`
  ;[1 1 1] Account Refresh Button
  (goto _label_2))

(event `self.ReceiveEndPlay`
  (params (EndPlayReason :type "EEndPlayReason Enum" :default "Destroyed"))
  (bind _returnvalue (subsystem `VivoxSubsystem`))
  (bind _username (`self.Username`))
  ;[1 1 1] Comment
  (`VivoxSubsystem.LeaveChannel` _returnvalue _username (`self.Channelname`) false)
  (`VivoxSubsystem.SignOut` _returnvalue _username))

(event `OnLeaveChannelClicked_Event`
  (params (DeleteChannel :type Boolean))
  ;[1 1 1] Leave Channel
  (bind _returnvalue (`VivoxSubsystem.LeaveChannel` (subsystem `VivoxSubsystem`) (`self.Username`) (`self.Channelname`) DeleteChannel))
  (`TextBlock.SetText` (`/InoVivox/UI/WBP_IV_Main.TB_ChannelLog` (`self.WBP_Vivox_Main_Ref`)) (`KismetTextLibrary.Conv_StringToText` (`KismetStringLibrary.Concat_StrStr` "leave channel " (select `bool` _returnvalue :`false` "failed" :`true` "success")))))

(event `OnSignoutClicked_Event`
  ;[1 1 1] Signout
  (bind _returnvalue (`VivoxSubsystem.SignOut` (subsystem `VivoxSubsystem`) (`self.Username`)))
  (`TextBlock.SetText` (`/InoVivox/UI/WBP_IV_Main.TB_AccountLog` (`self.WBP_Vivox_Main_Ref`)) (`KismetTextLibrary.Conv_StringToText` (`KismetStringLibrary.Concat_StrStr` "signout is started with error code " (`KismetStringLibrary.Conv_BoolToString` _returnvalue)))))

(event `Key|V`
  (params (Key :type "Key Structure"))
  (bind _channelname (`self.Channelname`))
  (bind _returnvalue (select `bool` (`self.IsTalking`) :`true` "Single" :!type "TransmissionMode Enum"))
  ;[1 1 1] SetTransmissionMode
  (:`Pressed`
    (set `self.IsTalking` true)
    (`VivoxSubsystem.SetTransmissionMode` (subsystem `VivoxSubsystem`) (`self.Username`) _channelname _returnvalue :!label _label_4)
    (`KismetSystemLibrary.PrintString` (`KismetStringLibrary.Concat_StrStr` "set transmission mode to " (`|GetEnumeratorNameAsString` _returnvalue) " for " _channelname) true true (struct :`G` 0.66 :`B` 1.0 :`A` 1.0) 10.0))
  (:`Released`
    (set `self.IsTalking` false)
    (goto _label_4)))

(fn `NewFunction`
  (params (A :type String))
  (returns (B :type String))
  (bind _returnvalue (`KismetStringLibrary.Concat_StrStr` "exampleuser" "11"))
  (return (select `bool` (`KismetStringLibrary.EqualEqual_StrStr` A _returnvalue) :`false` _returnvalue :`true` (`KismetStringLibrary.Concat_StrStr` "exampleuser" "22"))))

(fn `UserConstructionScript`)